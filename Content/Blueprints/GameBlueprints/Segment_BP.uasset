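; Segment_BP is a track segment actor that exposes lane points and spawn positions laid out as child components.
; At construction, SetupLanes gathers the direct children of the Lanes component into LanePointArray.
; GetSpawnPos treats the Rows component as a two-level grid, returning the world location of the child at a given row and lane index.
; The event graph holds no logic.
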(event EventBeginPlay)

(event Collision|EventActorBeginOverlap
  (params (OtherActor :type Actor%20Object%20Reference)))

(event EventTick
  (params (DeltaSeconds :type Float%20%28single-precision%29)))

(fn ConstructionScript
  (CallFunction|SetupLanes))

(fn SetupLanes
  (for _array_element (Components|GetChildrenComponents (Variables|Default|GetLanes) false)
    (Utilities|Array|Add (Variables|LanePositions|GetLanePointArray) _array_element)))

(fn GetSpawnPos
  (params (Row :type Integer) (RowLane :type Integer))
  (return (Transformation|GetWorldLocation (Components|GetChildComponent (Components|GetChildComponent (Variables|RowPositions|GetRows) Row) RowLane))))