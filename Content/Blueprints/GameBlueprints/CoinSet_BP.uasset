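; CoinSet_BP is a reusable group of Coin_BP child actors that is enabled for a given lane or disabled as a unit.
; On BeginPlay it caches the children of DefaultPositions as position markers.
; Enabling stores the lane, reactivates each coin, resets rotations, snaps coins back to their markers by index and gives each successive coin an incremented Pitch.
; Disabling deactivates the coins instead of destroying them.
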(event EventBeginPlay
  (CallFunction|SetupDefaultPositions))

(fn ConstructionScript)

(fn DisableCoinSet
  (for _array_element (Actor|GetAllChildActors true)
    (bind _ascoin_bp (Utilities|Casting|CastToCoin_BP _array_element))
    (CallFunction|DisableActor _ascoin_bp)))

(fn EnableCoinSet
  (params (CurrentLane :type Integer))
  (Variables|Default|SetCurrentLane CurrentLane)
  (for (_array_element _array_index) (Actor|GetAllChildActors true)
    (bind _ascoin_bp (Utilities|Casting|CastToCoin_BP _array_element))
    (CallFunction|EnableActor _ascoin_bp true true)
    (Transformation|SetActorRotation _ascoin_bp)
    (CallFunction|ResetPositions)
    (Variables|/Game/Blueprints/GameBlueprints/Coin_BP.Coin_BP_C|SetPitch _ascoin_bp (+ (* (Math|Conversions|ToFloat(Integer) _array_index) (Variables|Default|GetPitchIncrement)) (Variables|Default|GetDefaultPitch)))))

(fn ResetPositions
  (for (_array_element _array_index) (Actor|GetAllChildActors true)
    (bind _ascoin_bp (Utilities|Casting|CastToCoin_BP _array_element))
    (Transformation|SetActorLocation _ascoin_bp (Transformation|GetWorldLocation (Utilities|Array|Get(acopy) (Variables|Default|GetDefaultPositionArray) _array_index)) false false)))

(fn SetupDefaultPositions
  (for _array_element (Components|GetChildrenComponents (Variables|Default|GetDefaultPositions) false)
    (Utilities|Array|Add (Variables|Default|GetDefaultPositionArray) _array_element)))