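; PowerUp_BP is a power-up actor that spins in place and provides a collect sound.
; Tick advances its yaw by RotateSpeed scaled by delta time, keeping roll and pitch unchanged.
; PlayCollectSound plays the Powerup sound at the actor's location using its Volume and Pitch variables.
; The Blueprint itself holds no overlap or pickup logic, and nothing in it calls PlayCollectSound.
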(event EventTick
  (params (DeltaSeconds :type Float%20%28single-precision%29))
  (bind _returnvalue (Transformation|GetActorRotation))
  (bind (_roll _pitch _yaw) (Math|Rotator|BreakRotator _returnvalue))
  ;[1 1 1] Rotate
  (Transformation|SetActorRotation (Math|Rotator|MakeRotator _roll _pitch (+ _yaw (* (Variables|Default|GetRotateSpeed) DeltaSeconds)))))

(fn ConstructionScript)

(fn PlayCollectSound
  (Audio|PlaySoundatLocation "/Game/SFX/FX/powerup.powerup" (Transformation|GetActorLocation) "0, 0, 0" (Variables|Default|GetVolume) (Variables|Default|GetPitch) 0.0 0 0 0))