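; Manages a pool of power-ups and places them on upcoming track segments in a lane-based level.
; Initialize pre-spawns the PowerUp_BP actors and disables them into an available list.
; SpawnPowerUp picks a lane clear of the next segment's vertical obstacle and coin set, or matches a horizontal obstacle's row.
; It then moves and enables the first pooled power-up, assigns it to that segment and sets the spawned flag.
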(event EventBeginPlay)

(fn ConstructionScript)

(fn Initialize
  ;[1 1 1] Init PowerUps
  (for _index (range 0 (Variables|Default|GetTotalPowerUps))
    (bind _returnvalue (Game|SpawnActorfromClass "/Game/Blueprints/GameBlueprints/PowerUp_BP.PowerUp_BP_C" (Variables|Default|GetDefaultTransform) "Undefined" 0 0))
    (Utilities|Array|Add (Variables|Default|GetPowerUpsArray) _returnvalue)
    (CallFunction|AddtoAvailablePowerUpArray _returnvalue)))

(fn AddtoAvailablePowerUpArray
  (params (PowerUpToAdd :type Power%20Up%20BP%20Object%20Reference))
  (bind _aspower_up_bp (Utilities|Casting|CastToPowerUp_BP PowerUpToAdd))
  (Utilities|Array|Add (Variables|Default|GetAvailablePowerUpsArray) _aspower_up_bp)
  (CallFunction|DisableActor _aspower_up_bp)
  (Variables|Default|SetPowerUpIsSpawned false))

(fn RemovefromAvailablePowerUpArray
  (params (PowerUpToRemove :type Power%20Up%20BP%20Object%20Reference))
  (Utilities|Array|RemoveItem (Variables|Default|GetAvailablePowerUpsArray) PowerUpToRemove))

(fn SpawnPowerUp
  (bind _segmentmanagerref (Variables|Default|GetSegmentManagerRef))
  (bind _availablepowerupsarray (Variables|Default|GetAvailablePowerUpsArray))
  (bind _output (Utilities|Array|Get(acopy) _availablepowerupsarray))
  (bind _nextsegment (Variables|/Game/Blueprints/GameBlueprints/SegmentManager_BP.SegmentManager_BP_C|GetNextSegment _segmentmanagerref))
  (bind _activeobstacle (Variables|/Game/Blueprints/GameBlueprints/Segment_BP.Segment_BP_C|GetActiveObstacle _nextsegment))
  (bind _activecoinset (Variables|/Game/Blueprints/GameBlueprints/Segment_BP.Segment_BP_C|GetActiveCoinSet _nextsegment))
  ;[1 1 1] Checking for Obstacles and Coins
  (bind _asvertical_obstacle_bp (Utilities|Casting|CastToVerticalObstacle_BP _activeobstacle)
    (:then
      (LocalVariables|SetObstacleLane (Variables|/Game/Blueprints/GameBlueprints/VerticalObstacle_BP.VerticalObstacle_BP_C|GetCurrentLane _asvertical_obstacle_bp))
      (bind _ascoin_set_bp (Utilities|Casting|CastToCoinSet_BP _activecoinset)
        (:then
          (LocalVariables|SetCoinSetLane (Variables|/Game/Blueprints/GameBlueprints/CoinSet_BP.CoinSet_BP_C|GetCurrentLane _ascoin_set_bp))
          ;[1 1 1] If Obstacle and Coin set are both active on segment
          (bind _output_get (LocalVariables|SetLaneToSpawn 0))
          (while (or (== _output_get (LocalVariables|GetObstacleLane)) (== _output_get (LocalVariables|GetCoinSetLane)))
            (Math|Integer|IncrementInt (LocalVariables|GetLaneToSpawn))))
        (:CastFailed
          ;[1 1 1] If Obstacle only is active on segment
          (bind _output_get_2 (LocalVariables|SetLaneToSpawn (Math|Random|RandomInteger 3)))
          (while (== _output_get_2 (LocalVariables|GetObstacleLane))
            (LocalVariables|SetLaneToSpawn (Math|Random|RandomInteger 3))))))
    (:CastFailed
      ;[1 1 1] Make PowerUp match horizontal obstacle row
      (bind _ashorizontal_obstacle_bp (Utilities|Casting|CastToHorizontalObstacle_BP _activeobstacle)
        (:then
          (LocalVariables|SetRowToSpawn (Variables|/Game/Blueprints/GameBlueprints/HorizontalObstacle_BP.HorizontalObstacle_BP_C|GetCurrentRow _ashorizontal_obstacle_bp)))
        (:CastFailed
          _))
      (bind _ascoin_set_bp_2 (Utilities|Casting|CastToCoinSet_BP _activecoinset)
        (:then
          (LocalVariables|SetCoinSetLane (Variables|/Game/Blueprints/GameBlueprints/CoinSet_BP.CoinSet_BP_C|GetCurrentLane _ascoin_set_bp_2))
          ;[1 1 1] If Coin Set only is active on segment
          (bind _output_get_3 (LocalVariables|SetLaneToSpawn (Math|Random|RandomInteger 3)))
          (while (== _output_get_3 (LocalVariables|GetCoinSetLane))
            (LocalVariables|SetLaneToSpawn (Math|Random|RandomInteger 3))))
        (:CastFailed
          ;[1 1 1] If no Obstacle or Coin Set is active
          (LocalVariables|SetLaneToSpawn (Math|Random|RandomInteger 3))))))
  ;[1 1 1] Spawn Logic
  (bind _position (Default|GetSpawnPos (Variables|/Game/Blueprints/GameBlueprints/SegmentManager_BP.SegmentManager_BP_C|GetNextSegment (Variables|Default|GetSegmentManagerRef)) (LocalVariables|GetRowToSpawn) (LocalVariables|GetLaneToSpawn)))
  (Transformation|SetActorLocation _output _position false false)
  (CallFunction|EnableActor _output true true)
  (bind _output_get_4 (Variables|/Game/Blueprints/GameBlueprints/Segment_BP.Segment_BP_C|SetActivePowerup (Variables|/Game/Blueprints/GameBlueprints/SegmentManager_BP.SegmentManager_BP_C|GetNextSegment (Variables|Default|GetSegmentManagerRef)) _output))
  (CallFunction|RemovefromAvailablePowerUpArray _output_get_4)
  (Variables|Default|SetPowerUpIsSpawned true))

(fn Reset
  (Variables|Default|SetPowerUpIsSpawned false))