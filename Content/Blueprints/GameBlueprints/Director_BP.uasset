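; Director actor that bootstraps a segment-based game run and owns its gameplay and game-over UI.
; On BeginPlay it spawns the segment, obstacle, coin and power-up managers, passing the segment manager into the other three at spawn.
; It cross-links managers and player, then initializes them in order: obstacles, coins, power-ups, segments, player.
; It creates score and game-over widgets and exposes functions to toggle between them.
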(event EventBeginPlay
  (bind _defaulttransform (Variables|Default|GetDefaultTransform))
  ;[1 1 1] Setup Segment Manager
  (bind _returnvalue (Game|SpawnActorfromClass "/Game/Blueprints/GameBlueprints/SegmentManager_BP.SegmentManager_BP_C" _defaulttransform "Undefined" 0 0))
  (bind _output_get (Variables|Default|SetSegmentManager _returnvalue))
  ;[1 1 1] Setup Obstacle Manager
  (bind _returnvalue_2 (Game|SpawnActorfromClass "/Game/Blueprints/GameBlueprints/ObstacleManager_BP.ObstacleManager_BP_C" _defaulttransform "Undefined" 0 _output_get 0))
  (bind _output_get_2 (Variables|Default|SetObstacleManager _returnvalue_2))
  ;[1 1 1] Setup Coin Manager
  (bind _returnvalue_3 (Game|SpawnActorfromClass "/Game/Blueprints/GameBlueprints/CoinManager_BP.CoinManager_BP_C" _defaulttransform "Undefined" 0 _output_get 0))
  (bind _output_get_3 (Variables|Default|SetCoinManager _returnvalue_3))
  ;[1 1 1] Setup PowerUp Manager
  (bind _returnvalue_4 (Game|SpawnActorfromClass "/Game/Blueprints/GameBlueprints/PowerUpManager_BP.PowerUpManager_BP_C" _defaulttransform "Undefined" 0 _output_get 0))
  (bind _output_get_4 (Variables|Default|SetPowerUpManager _returnvalue_4))
  ;[1 1 1] Set Player Ref
  (bind _asplayer_bp (Utilities|Casting|CastToPlayer_BP (Game|Player|GetPlayerPawn 0)))
  (bind _output_get_5 (Variables|Default|SetPlayerRef _asplayer_bp))
  ;[1 1 1] Give Manager Refs to Segment Manager
  (Default|SetManagerRefs _output_get _output_get_2 _output_get_3 _output_get_4 _output_get_5)
  ;[1 1 1] Give Segment Manager Ref and Director ref to Player
  (Default|SetManagerRefs _output_get_5 _output_get self)
  (CallFunction|InitializeManagers)
  (CallFunction|SetupWidgets))

(fn ConstructionScript)

(fn InitializeManagers
  ;[1 1 1] Init Obstacle Manager
  (Default|Initialize (Variables|Default|GetObstacleManager))
  ;[1 1 1] Init Coin Manager
  (Default|Initialize (Variables|Default|GetCoinManager))
  ;[1 1 1] Init PowerUp Manager
  (Default|Initialize (Variables|Default|GetPowerUpManager))
  ;[1 1 1] Init Segment Manager
  (Default|Initialize (Variables|Default|GetSegmentManager))
  ;[1 1 1] Init Player
  (Default|Initialize (Variables|Default|GetPlayerRef)))

(fn SetupWidgets
  (Utilities|FlowControl|Sequence
    (:then_0
      ;[1 1 1] Creating Widgets
      (bind _returnvalue (UserInterface|CreateWidget "/Game/Blueprints/GameBlueprints/Score_Widget.Score_Widget_C"))
      (bind _output_get (Variables|Default|SetScoreWidget _returnvalue))
      (UserInterface|Viewport|AddtoViewport _output_get 0))
    (:then_1
      (bind _returnvalue_2 (UserInterface|CreateWidget "/Game/Blueprints/GameBlueprints/GameOver_Widget.GameOver_Widget_C"))
      (bind _output_get_2 (Variables|Default|SetGameOverWidget _returnvalue_2))
      (UserInterface|Viewport|AddtoViewport _output_get_2 0)
      (Widget|SetVisibility _output_get_2 "Hidden"))))

(fn ActivateGameOverWidget
  (bind _gameoverwidget (Variables|Default|GetGameOverWidget))
  (Default|SetScoreString _gameoverwidget)
  (Widget|SetVisibility _gameoverwidget "Visible")
  (Widget|SetVisibility (Variables|Default|GetScoreWidget) "Hidden"))

(fn ActivateGameplayWidget
  (Widget|SetVisibility (Variables|Default|GetGameOverWidget) "Hidden")
  (Widget|SetVisibility (Variables|Default|GetScoreWidget) "Visible"))