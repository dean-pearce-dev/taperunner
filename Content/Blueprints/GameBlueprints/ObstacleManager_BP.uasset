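; Obstacle manager that pools horizontal and vertical obstacles and places them on track segments.
; Initialize pre-spawns both types, and AddToAvailableObstacleArray disables each and files it in its type's available array.
; SpawnObstacle randomly picks a type, moves the first pooled one onto SegmentManagerRef's NextSegment, enables it and removes it from the pool.
; Vertical obstacles get a random row and lane; horizontal ones get a random row in a fixed lane.
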(fn ConstructionScript)

(fn AddtoAvailableObstacleArray
  (params (Obstacle%20to%20Add :type Obstacle%20BP%20Object%20Reference))
  (bind _ashorizontal_obstacle_bp (Utilities|Casting|CastToHorizontalObstacle_BP Obstacle%20to%20Add)
    (:then
      (Utilities|Array|Add (Variables|Default|GetAvailableHorizontalObstacles) _ashorizontal_obstacle_bp)
      (CallFunction|DisableActor _ashorizontal_obstacle_bp))
    (:CastFailed
      (bind _asvertical_obstacle_bp (Utilities|Casting|CastToVerticalObstacle_BP Obstacle%20to%20Add))
      (Utilities|Array|Add (Variables|Default|GetAvailableVerticalObstacles) _asvertical_obstacle_bp)
      (CallFunction|DisableActor _asvertical_obstacle_bp))))

(fn RemovefromAvailableObstacleArray
  (params (Obstacle%20to%20Remove :type Obstacle%20BP%20Object%20Reference))
  (bind _ashorizontal_obstacle_bp (Utilities|Casting|CastToHorizontalObstacle_BP Obstacle%20to%20Remove)
    (:then
      (Utilities|Array|RemoveItem (Variables|Default|GetAvailableHorizontalObstacles) _ashorizontal_obstacle_bp))
    (:CastFailed
      (bind _asvertical_obstacle_bp (Utilities|Casting|CastToVerticalObstacle_BP Obstacle%20to%20Remove))
      (Utilities|Array|RemoveItem (Variables|Default|GetAvailableVerticalObstacles) _asvertical_obstacle_bp))))

(fn SpawnObstacle
  (bind _segmentmanagerref (Variables|Default|GetSegmentManagerRef))
  (bind _availableverticalobstacles (Variables|Default|GetAvailableVerticalObstacles))
  (bind _availablehorizontalobstacles (Variables|Default|GetAvailableHorizontalObstacles))
  (bind _segmentmanagerref_2 (Variables|Default|GetSegmentManagerRef))
  (bind _output (Utilities|Array|Get(acopy) _availableverticalobstacles))
  (bind _output_2 (Utilities|Array|Get(acopy) _availablehorizontalobstacles))
  (bind _nextsegment (Variables|/Game/Blueprints/GameBlueprints/SegmentManager_BP.SegmentManager_BP_C|GetNextSegment _segmentmanagerref))
  (bind _nextsegment_2 (Variables|/Game/Blueprints/GameBlueprints/SegmentManager_BP.SegmentManager_BP_C|GetNextSegment _segmentmanagerref_2))
  (switch int (Math|Random|RandomInteger 2)
    (:0
      ;[1 1 1] Spawn Vertical Obstacle
      (bind _output_get (LocalVariables|SetVerticalObstacleLane (Math|Random|RandomInteger 3)))
      (bind _position (Default|GetSpawnPos _nextsegment_2 (Math|Random|RandomInteger 3) _output_get))
      (Transformation|SetActorLocation _output _position false false)
      (CallFunction|EnableActor _output false true)
      (Variables|/Game/Blueprints/GameBlueprints/Segment_BP.Segment_BP_C|SetActiveObstacle _nextsegment_2 _output)
      (Variables|/Game/Blueprints/GameBlueprints/VerticalObstacle_BP.VerticalObstacle_BP_C|SetCurrentLane _output (LocalVariables|GetVerticalObstacleLane))
      (CallFunction|RemovefromAvailableObstacleArray _output))
    (:1
      ;[1 1 1] Spawn Horizontal Obstacle
      (bind _output_get_2 (Variables|/Game/Blueprints/GameBlueprints/HorizontalObstacle_BP.HorizontalObstacle_BP_C|SetCurrentRow _output_2 (Math|Random|RandomInteger 3)))
      (bind _position_2 (Default|GetSpawnPos _nextsegment _output_get_2 1))
      (Transformation|SetActorLocation _output_2 _position_2 false false)
      (CallFunction|EnableActor _output_2 false true)
      (bind _output_get_3 (Variables|/Game/Blueprints/GameBlueprints/Segment_BP.Segment_BP_C|SetActiveObstacle _nextsegment _output_2))
      (CallFunction|RemovefromAvailableObstacleArray _output_get_3))))

(fn Initialize
  (bind _defaulttransform (Variables|Default|GetDefaultTransform))
  ;[1 1 1] Init Obstacles
  (for _index (range 0 (Variables|Default|GetTotalHorizontalObstacles))
    (bind _returnvalue (Game|SpawnActorfromClass "/Game/Blueprints/GameBlueprints/HorizontalObstacle_BP.HorizontalObstacle_BP_C" _defaulttransform "Undefined" 0 0))
    (CallFunction|AddtoAvailableObstacleArray _returnvalue))
  (for _index_2 (range 0 (Variables|Default|GetTotalVerticalObstacles))
    (bind _returnvalue_2 (Game|SpawnActorfromClass "/Game/Blueprints/GameBlueprints/VerticalObstacle_BP.VerticalObstacle_BP_C" _defaulttransform "Undefined" 0 0))
    (CallFunction|AddtoAvailableObstacleArray _returnvalue_2)))