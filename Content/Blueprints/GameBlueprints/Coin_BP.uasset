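; Coin Blueprint that spins around its yaw axis and can fly toward the player pawn.
; StartFlyTo records the coin's position and resets the lerp, then Tick moves it toward the player's live location at FlyToSpeed until alpha reaches one.
; PlayCollectSound plays the collect sound at the coin with a variable pitch; nothing in this Blueprint calls it or StartFlyTo, or destroys the coin.
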(event EventBeginPlay
  ;[1 1 1] Set Player Ref
  (bind _asplayer_bp (Utilities|Casting|CastToPlayer_BP (Game|Player|GetPlayerPawn 0)))
  (Variables|Default|SetPlayerRef _asplayer_bp))

(event EventTick
  (params (DeltaSeconds :type Float%20%28single-precision%29))
  (bind _returnvalue (Transformation|GetActorRotation))
  (bind (_roll _pitch _yaw) (Math|Rotator|BreakRotator _returnvalue))
  ;[1 1 1] Rotate
  (Transformation|SetActorRotation (Math|Rotator|MakeRotator _roll _pitch (+ _yaw (* (Variables|Default|GetRotateSpeed) DeltaSeconds))))
  (if (Variables|Default|GetIsFlyingToPlayer)
    (CallFunction|FlytoPlayer)))

(fn ConstructionScript)

(fn PlayCollectSound
  (Audio|PlaySoundatLocation "/Game/SFX/FX/collect.collect" (Transformation|GetActorLocation) "0, 0, 0" 0.6 (Variables|Default|GetPitch) 0.0 0 0 0))

(fn FlytoPlayer
  (Transformation|SetActorLocation (Math|Vector|Lerp(Vector) (Variables|Default|GetLerpFrom) (Transformation|GetActorLocation (Variables|Default|GetPlayerRef)) (Variables|Default|GetLerpValue)) false false)
  (CallFunction|LerpIncrease))

(fn StartFlyto
  (Variables|Default|SetIsFlyingToPlayer true)
  (Variables|Default|SetLerpFrom (Transformation|GetActorLocation))
  (Variables|Default|SetLerpValue 0.0))

(fn LerpIncrease
  (Variables|Default|SetLerpValue (+ (Variables|Default|GetLerpValue) (* (Variables|Default|GetFlyToSpeed) (Utilities|Time|GetWorldDeltaSeconds))))
  (if (>= (Variables|Default|GetLerpValue) 1.0)
    (Variables|Default|SetIsFlyingToPlayer false)))