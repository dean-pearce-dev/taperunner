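; Coin manager that pools straight and curved coin sets and places them on the next track segment from SegmentManagerRef.
; Initialize pre-spawns both types into disabled pools; spawning enables the first available set, assigns it to the segment and removes it from its pool.
; Horizontal obstacles get a curved set on their row; otherwise the type is random, in a random lane that avoids any vertical obstacle.
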(fn ConstructionScript)

(fn AddtoAvailableCoinSetArray
  (params (Coin%20Set%20to%20Add :type Coin%20Set%20BP%20Object%20Reference))
  (bind _ascurved_coin_set_bp (Utilities|Casting|CastToCurvedCoinSet_BP Coin%20Set%20to%20Add)
    (:then
      (Utilities|Array|Add (Variables|Default|GetAvailableCurvedCoinSetArray) _ascurved_coin_set_bp)
      (Default|DisableCoinSet Coin%20Set%20to%20Add)
      (CallFunction|DisableActor Coin%20Set%20to%20Add))
    (:CastFailed
      (bind _asstraight_coin_set_bp (Utilities|Casting|CastToStraightCoinSet_BP Coin%20Set%20to%20Add))
      (Utilities|Array|Add (Variables|Default|GetAvailableStraightCoinSetArray) _asstraight_coin_set_bp)
      (Default|DisableCoinSet Coin%20Set%20to%20Add)
      (CallFunction|DisableActor Coin%20Set%20to%20Add))))

(fn RemovefromAvailableCoinArray
  (params (Coin%20Set%20to%20Remove :type Coin%20Set%20BP%20Object%20Reference))
  (bind _ascurved_coin_set_bp (Utilities|Casting|CastToCurvedCoinSet_BP Coin%20Set%20to%20Remove)
    (:then
      (Utilities|Array|RemoveItem (Variables|Default|GetAvailableCurvedCoinSetArray) _ascurved_coin_set_bp))
    (:CastFailed
      (bind _asstraight_coin_set_bp (Utilities|Casting|CastToStraightCoinSet_BP Coin%20Set%20to%20Remove))
      (Utilities|Array|RemoveItem (Variables|Default|GetAvailableStraightCoinSetArray) _asstraight_coin_set_bp))))

(fn SpawnCoinSet
  (bind _segmentmanagerref (Variables|Default|GetSegmentManagerRef))
  (bind _nextsegment (Variables|/Game/Blueprints/GameBlueprints/SegmentManager_BP.SegmentManager_BP_C|GetNextSegment _segmentmanagerref))
  (bind _activeobstacle (Variables|/Game/Blueprints/GameBlueprints/Segment_BP.Segment_BP_C|GetActiveObstacle _nextsegment))
  ;[1 1 1] Spawn Curved Coin Set if there's a Horizontal Obstacle
  (bind _ashorizontal_obstacle_bp (Utilities|Casting|CastToHorizontalObstacle_BP _activeobstacle)
    (:then
      (bind _output_get (LocalVariables|SetLaneToSpawn (Math|Random|RandomInteger 3)))
      (bind _position (Default|GetSpawnPos (Variables|/Game/Blueprints/GameBlueprints/SegmentManager_BP.SegmentManager_BP_C|GetNextSegment (Variables|Default|GetSegmentManagerRef)) (Variables|/Game/Blueprints/GameBlueprints/HorizontalObstacle_BP.HorizontalObstacle_BP_C|GetCurrentRow _ashorizontal_obstacle_bp) _output_get))
      (CallFunction|SpawnCurvedCoinSet _position _output_get))
    (:CastFailed
      ;[1 1 1] If there's a vertical obstacle, make sure coin set doesn't spawn on same lane
      (bind _asvertical_obstacle_bp (Utilities|Casting|CastToVerticalObstacle_BP _activeobstacle)
        (:then
          (bind _output_get_2 (LocalVariables|SetLaneToSpawn (Math|Random|RandomInteger 3)))
          (while (== _output_get_2 (Variables|/Game/Blueprints/GameBlueprints/VerticalObstacle_BP.VerticalObstacle_BP_C|GetCurrentLane _asvertical_obstacle_bp))
            (LocalVariables|SetLaneToSpawn (Math|Random|RandomInteger 3)))
          (bind _position_2 (Default|GetSpawnPos (Variables|/Game/Blueprints/GameBlueprints/SegmentManager_BP.SegmentManager_BP_C|GetNextSegment (Variables|Default|GetSegmentManagerRef)) 1 (LocalVariables|GetLaneToSpawn)))
          (switch int (Math|Random|RandomInteger 2)
            (:0
              (CallFunction|SpawnStraightCoinSet _position_2 (LocalVariables|GetLaneToSpawn)))
            (:1
              (CallFunction|SpawnCurvedCoinSet _position_2 (LocalVariables|GetLaneToSpawn)))))
        (:CastFailed
          ;[1 1 1] When no obstacle, spawn anywhere, and any type of coin set
          (bind _output_get_3 (LocalVariables|SetLaneToSpawn (Math|Random|RandomInteger 3)))
          (bind _position_3 (Default|GetSpawnPos (Variables|/Game/Blueprints/GameBlueprints/SegmentManager_BP.SegmentManager_BP_C|GetNextSegment (Variables|Default|GetSegmentManagerRef)) 1 _output_get_3))
          (switch int (Math|Random|RandomInteger 2)
            (:0
              (CallFunction|SpawnStraightCoinSet _position_3 _output_get_3))
            (:1
              (CallFunction|SpawnCurvedCoinSet _position_3 _output_get_3))))))))

(fn SpawnStraightCoinSet
  (params (Position%20to%20Spawn :type Vector) (CurrentLane :type Integer))
  (bind _availablestraightcoinsetarray (Variables|Default|GetAvailableStraightCoinSetArray))
  (bind _output (Utilities|Array|Get(acopy) _availablestraightcoinsetarray))
  (Transformation|SetActorLocation _output Position%20to%20Spawn false false)
  (Default|EnableCoinSet _output CurrentLane)
  (CallFunction|EnableActor _output false false)
  (bind _output_get (Variables|/Game/Blueprints/GameBlueprints/Segment_BP.Segment_BP_C|SetActiveCoinSet (Variables|/Game/Blueprints/GameBlueprints/SegmentManager_BP.SegmentManager_BP_C|GetNextSegment (Variables|Default|GetSegmentManagerRef)) _output))
  (CallFunction|RemovefromAvailableCoinArray _output_get))

(fn SpawnCurvedCoinSet
  (params (Position%20to%20Spawn :type Vector) (CurrentLane :type Integer))
  (bind _availablecurvedcoinsetarray (Variables|Default|GetAvailableCurvedCoinSetArray))
  (bind _output (Utilities|Array|Get(acopy) _availablecurvedcoinsetarray))
  (Transformation|SetActorLocation _output Position%20to%20Spawn false false)
  (Default|EnableCoinSet _output CurrentLane)
  (CallFunction|EnableActor _output false false)
  (bind _output_get (Variables|/Game/Blueprints/GameBlueprints/Segment_BP.Segment_BP_C|SetActiveCoinSet (Variables|/Game/Blueprints/GameBlueprints/SegmentManager_BP.SegmentManager_BP_C|GetNextSegment (Variables|Default|GetSegmentManagerRef)) _output))
  (CallFunction|RemovefromAvailableCoinArray _output_get))

(fn Initialize
  (Utilities|FlowControl|Sequence
    (:then_0
      ;[1 1 1] Init CoinSets
      (for _index (range 0 (Variables|Default|GetTotalCoinSets))
        (bind _returnvalue (Game|SpawnActorfromClass "/Game/Blueprints/GameBlueprints/StraightCoinSet_BP.StraightCoinSet_BP_C" (Variables|Default|GetDefaultTransform) "Undefined" 0 0))
        (Utilities|Array|Add (Variables|Default|GetStraightCoinSetArray) _returnvalue)
        (CallFunction|AddtoAvailableCoinSetArray _returnvalue)))
    (:then_1
      ;[1 1 1] Init CurvedCoinSets
      (for _index_2 (range 0 (Variables|Default|GetTotalCurvedCoinSets))
        (bind _returnvalue_2 (Game|SpawnActorfromClass "/Game/Blueprints/GameBlueprints/CurvedCoinSet_BP.CurvedCoinSet_BP_C" (Variables|Default|GetDefaultTransform) "Undefined" 0 0))
        (Utilities|Array|Add (Variables|Default|GetCurvedCoinSetArray) _returnvalue_2)
        (CallFunction|AddtoAvailableCoinSetArray _returnvalue_2)))))