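; Segment manager for an endless-runner style track, pooling straight segments and chaining them end to end.
; Initialize spawns the segment pool and fills the queue, leaving the first segments free of objects.
; SetupNextSegment recycles flagged segments with their obstacle, coin set and power-up, then places a pooled segment at the queue's last end point.
; It randomly requests objects from their managers, allowing power-ups only when none is spawned or active.
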(fn ConstructionScript)

(fn SetupNextSegment
  (params (IsInitialSpawnPhase :type Boolean) (IgnoreObjectSpawns :type Boolean))
  (bind _powerupmanagerref (Variables|Default|GetPowerUpManagerRef))
  (if IsInitialSpawnPhase
    _
    (else
      ;[1 1 1] Flagging Segments to despawn, and removing from queue.
      (CallFunction|DespawnFlaggedSegments)
      (CallFunction|FlagSegmentforDespawn (Variables|Segments|GetCurrentSegment))
      (Variables|Segments|SetCurrentSegment (Utilities|Array|Get(acopy) (Variables|Segments|GetQueuedSegmentArray)))))
  (bind _spawn_point (CallFunction|GetSegmentSpawnPoint))
  (LocalVariables|SetSpawnPoint _spawn_point)
  ;[1 1 1] Get Available Segment for Next Segment
  (bind _output_get (Variables|Segments|SetNextSegment (Utilities|Array|Get(acopy) (Variables|Segments|GetStraightSegmentAvailableArray))))
  ;[1 1 1] Setup Next Segment
  (bind _enabled_segment (CallFunction|EnableSegment _output_get))
  (Transformation|SetActorLocation _enabled_segment (LocalVariables|GetSpawnPoint) false false)
  (CallFunction|AddtoSegmentQueue _enabled_segment)
  (if (not IgnoreObjectSpawns)
    (Utilities|FlowControl|Sequence
      (:then_0
        ;[1 1 1] Randomise to spawn obstacle
        (if (> (Math|Random|RandomInteger 2) 0)
          (Default|SpawnObstacle (Variables|Default|GetObstacleManagerRef))))
      (:then_1
        ;[1 1 1] Randomise to spawn coin set
        (if (> (Math|Random|RandomInteger 2) 0)
          (Default|SpawnCoinSet (Variables|Default|GetCoinManagerRef))))
      (:then_2
        ;[1 1 1] Only spawn PowerUp if one isn't already spawned and if Player isn't powered up
        (if (not (or (Variables|/Game/Blueprints/GameBlueprints/PowerUpManager_BP.PowerUpManager_BP_C|GetPowerUpIsSpawned _powerupmanagerref) (Variables|/Game/Blueprints/GameBlueprints/Player_BP.Player_BP_C|GetIsPoweredUp (Variables|Default|GetPlayerRef))))
          ;[1 1 1] Randomise to spawn power up
          (if (> (Math|Random|RandomInteger 8) 6)
            (Default|SpawnPowerUp _powerupmanagerref)))))))

(fn AddtoAvailableSegmentArray
  (params (Segment%20to%20Add :type Segment%20BP%20Object%20Reference))
  (bind _asstraight_segment_bp (Utilities|Casting|CastToStraightSegment_BP Segment%20to%20Add))
  (Utilities|Array|Add (Variables|Segments|GetStraightSegmentAvailableArray) _asstraight_segment_bp)
  (Variables|/Game/Blueprints/GameBlueprints/Segment_BP.Segment_BP_C|SetFlaggedToDespawn _asstraight_segment_bp false)
  (CallFunction|DisableActor _asstraight_segment_bp))

(fn RemovefromAvailableSegmentArray
  (params (Segment%20to%20Remove :type Segment%20BP%20Object%20Reference))
  (bind _asstraight_segment_bp (Utilities|Casting|CastToStraightSegment_BP Segment%20to%20Remove))
  (Utilities|Array|RemoveItem (Variables|Segments|GetStraightSegmentAvailableArray) _asstraight_segment_bp))

(fn DespawnFlaggedSegments
  (for _array_element (Variables|Segments|GetSegmentArray)
    (if (Variables|/Game/Blueprints/GameBlueprints/Segment_BP.Segment_BP_C|GetFlaggedToDespawn _array_element)
      ;[1 1 1] Clear Obstacle
      (Default|AddtoAvailableObstacleArray (Variables|Default|GetObstacleManagerRef) (Variables|/Game/Blueprints/GameBlueprints/Segment_BP.Segment_BP_C|GetActiveObstacle _array_element))
      (Variables|/Game/Blueprints/GameBlueprints/Segment_BP.Segment_BP_C|SetActiveObstacle _array_element 0)
      ;[1 1 1] Clear Coin Set
      (Default|AddtoAvailableCoinSetArray (Variables|Default|GetCoinManagerRef) (Variables|/Game/Blueprints/GameBlueprints/Segment_BP.Segment_BP_C|GetActiveCoinSet _array_element))
      (Variables|/Game/Blueprints/GameBlueprints/Segment_BP.Segment_BP_C|SetActiveCoinSet _array_element 0)
      ;[1 1 1] Clear PowerUp
      (Default|AddtoAvailablePowerUpArray (Variables|Default|GetPowerUpManagerRef) (Variables|/Game/Blueprints/GameBlueprints/Segment_BP.Segment_BP_C|GetActivePowerup _array_element))
      (Variables|/Game/Blueprints/GameBlueprints/Segment_BP.Segment_BP_C|SetActivePowerup _array_element 0)
      (CallFunction|AddtoAvailableSegmentArray _array_element))))

(fn EnableSegment
  (params (Segment%20to%20Enable :type Segment%20BP%20Object%20Reference))
  (CallFunction|EnableActor Segment%20to%20Enable false false)
  (CallFunction|RemovefromAvailableSegmentArray Segment%20to%20Enable)
  (return Segment%20to%20Enable))

(fn AddtoSegmentQueue
  (params (Segment%20to%20Add :type Segment%20BP%20Object%20Reference))
  (Utilities|Array|Add (Variables|Segments|GetQueuedSegmentArray) Segment%20to%20Add))

(fn RemovefromSegmentQueue
  (params (Segment%20to%20Remove :type Segment%20BP%20Object%20Reference))
  (Utilities|Array|RemoveItem (Variables|Segments|GetQueuedSegmentArray) Segment%20to%20Remove))

(fn FlagSegmentforDespawn
  (params (Segment%20to%20Flag :type Segment%20BP%20Object%20Reference))
  (Variables|/Game/Blueprints/GameBlueprints/Segment_BP.Segment_BP_C|SetFlaggedToDespawn Segment%20to%20Flag true)
  (CallFunction|RemovefromSegmentQueue Segment%20to%20Flag))

(fn GetSegmentSpawnPoint
  (bind _queuedsegmentarray (Variables|Segments|GetQueuedSegmentArray))
  ;[1 1 1] Check if queue is empty for initial setup
  (if (== (Utilities|Array|Length (Variables|Segments|GetQueuedSegmentArray)) 0)
    (return "0, 0, 0")
    (else
      ;[1 1 1] Get Last segment in queue for spawn point
      (return (Transformation|GetWorldLocation (Variables|/Game/Blueprints/GameBlueprints/Segment_BP.Segment_BP_C|GetEndPoint (Utilities|Array|Get(acopy) _queuedsegmentarray (- (Utilities|Array|Length _queuedsegmentarray) 1))))))))

(fn Reset
  (CallFunction|ClearQueue)
  (CallFunction|InitSegments)
  (Default|Reset (Variables|Default|GetPowerUpManagerRef)))

(fn ClearQueue
  (for _array_element (Variables|Segments|GetSegmentArray)
    (CallFunction|FlagSegmentforDespawn _array_element))
  (CallFunction|DespawnFlaggedSegments))

(fn InitSegments
  (for _index (range 0 (Variables|Segments|GetTotalQueuedSegments))
    (if (< _index 2)
      (CallFunction|SetupNextSegment true true)
      (else
        (CallFunction|SetupNextSegment true false))))
  (bind _output_get (Variables|Segments|SetCurrentSegment (Utilities|Array|Get(acopy) (Variables|Segments|GetQueuedSegmentArray))))
  (CallFunction|FlagSegmentforDespawn _output_get)
  ;[1 1 1] Duplicate code, improve later
  (Variables|Segments|SetCurrentSegment (Utilities|Array|Get(acopy) (Variables|Segments|GetQueuedSegmentArray))))

(fn SetManagerRefs
  (params (ObstacleManager :type Obstacle%20Manager%20BP%20Object%20Reference) (CoinManager :type Coin%20Manager%20BP%20Object%20Reference) (PowerUpManager :type Power%20Up%20Manager%20BP%20Object%20Reference) (PlayerRef :type Player%20BP%20Object%20Reference))
  (Variables|Default|SetObstacleManagerRef ObstacleManager)
  (Variables|Default|SetCoinManagerRef CoinManager)
  (Variables|Default|SetPowerUpManagerRef PowerUpManager)
  (Variables|Default|SetPlayerRef PlayerRef))

(fn Initialize
  (Utilities|FlowControl|Sequence
    (:then_0
      ;[1 1 1] Init StraightSegments
      ;;[1 1 1] Create Segments
      (for _index (range 0 (Variables|Segments|GetTotalStraightSegments))
        (bind _returnvalue (Game|SpawnActorfromClass "/Game/Blueprints/GameBlueprints/StraightSegment_BP.StraightSegment_BP_C" (Variables|Default|GetDefaultTransform) "Undefined" 0 0))
        (Utilities|Array|Add (Variables|Segments|GetSegmentArray) _returnvalue)
        (CallFunction|AddtoAvailableSegmentArray _returnvalue)))
    (:then_1
      ;[1 1 1] Init Segment Queue
      (for _index_2 (range 0 (Variables|Segments|GetTotalQueuedSegments))
        (if (< _index_2 2)
          (CallFunction|SetupNextSegment true true)
          (else
            (CallFunction|SetupNextSegment true false))))
      (bind _output_get (Variables|Segments|SetCurrentSegment (Utilities|Array|Get(acopy) (Variables|Segments|GetQueuedSegmentArray))))
      (CallFunction|FlagSegmentforDespawn _output_get)
      ;;[1 1 1] Duplicate code, improve later
      (Variables|Segments|SetCurrentSegment (Utilities|Array|Get(acopy) (Variables|Segments|GetQueuedSegmentArray))))))